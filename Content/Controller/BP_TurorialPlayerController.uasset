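; Tutorial player controller that turns Enhanced Input actions into commands on its possessed BP_TurorialCharacter.
; On possession it casts and caches the pawn, and each input handler checks that reference before forwarding move, look, jump, gait and strafe calls.
; Walk toggles between walk and run and records the base speed, which releasing sprint restores.
; Strafe lasts while its input is held, then returns to neutral.
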(event `self.ReceivePossess`
  (params (PossessedPawn :type "Pawn Object Reference"))
  (`self.TryCacheCharacter`))

(event `EnhancedInput|/Game/Input/Actions/IA_Move`
  (params (ActionValue :type "Vector2D Structure") (ElapsedSeconds :type "Float (double-precision)") (TriggeredSeconds :type "Float (double-precision)") (InputAction :type "InputAction Object Reference" :default "/Game/Input/Actions/IA_Move.IA_Move"))
  (:`Triggered`
    (bind _poseesedcharacter (`self.PoseesedCharacter` :!label _label)
      (:`then`
        (`/Game/Blueprints/BP_TurorialCharacter.Move` _poseesedcharacter ActionValue))
      (:`else`)))
  (:`Canceled`
    (goto _label))
  (:`Completed`
    (goto _label)))

(event `EnhancedInput|/Game/Input/Actions/IA_Look`
  (params (ActionValue :type "Vector2D Structure") (ElapsedSeconds :type "Float (double-precision)") (TriggeredSeconds :type "Float (double-precision)") (InputAction :type "InputAction Object Reference" :default "/Game/Input/Actions/IA_Look.IA_Look"))
  (:`Triggered`
    (bind _poseesedcharacter (`self.PoseesedCharacter`)
      (:`then`
        (`Pawn.AddControllerYawInput` _poseesedcharacter ActionValue_X)
        (`Pawn.AddControllerPitchInput` _poseesedcharacter ActionValue_Y))
      (:`else`))))

(event `EnhancedInput|/Game/Input/Actions/IA_Jump`
  (params (ActionValue :type Boolean) (ElapsedSeconds :type "Float (double-precision)") (TriggeredSeconds :type "Float (double-precision)") (InputAction :type "InputAction Object Reference" :default "/Game/Input/Actions/IA_Jump.IA_Jump"))
  (:`Triggered`
    (bind _poseesedcharacter (`self.PoseesedCharacter`)
      (:`then`
        (`Character.Jump` _poseesedcharacter))
      (:`else`))))

(event `EnhancedInput|/Game/Input/Actions/IA_Walk`
  (params (ActionValue :type Boolean) (ElapsedSeconds :type "Float (double-precision)") (TriggeredSeconds :type "Float (double-precision)") (InputAction :type "InputAction Object Reference" :default "/Game/Input/Actions/IA_Walk.IA_Walk"))
  (bind _poseesedcharacter (`self.PoseesedCharacter`))
  (:`Triggered`
    (bind _poseesedcharacter_2 (`self.PoseesedCharacter`)
      (:`then`
        (if (== (`/Game/Blueprints/BP_TurorialCharacter.BP_SpeedTag` _poseesedcharacter_2) (struct :`TagName` "Motion.Speed.Walk"))
          (`/Game/Blueprints/BP_TurorialCharacter.BeginRun` _poseesedcharacter)
          (set `self.IsBaseSpeedWalk` false)
          (else
            (`/Game/Blueprints/BP_TurorialCharacter.BeginWalk` _poseesedcharacter)
            (set `self.IsBaseSpeedWalk` true))))
      (:`else`))))

(event `EnhancedInput|/Game/Input/Actions/IA_Sprint`
  (params (ActionValue :type Boolean) (ElapsedSeconds :type "Float (double-precision)") (TriggeredSeconds :type "Float (double-precision)") (InputAction :type "InputAction Object Reference" :default "/Game/Input/Actions/IA_Sprint.IA_Sprint"))
  (:`Started`
    (bind _poseesedcharacter (`self.PoseesedCharacter`)
      (:`then`
        (`/Game/Blueprints/BP_TurorialCharacter.BeginSprint` _poseesedcharacter))
      (:`else`)))
  (:`Canceled`
    (bind _poseesedcharacter_2 (`self.PoseesedCharacter` :!label _label_2)
      (:`then`
        (if (`self.IsBaseSpeedWalk`)
          (`/Game/Blueprints/BP_TurorialCharacter.BeginWalk` _poseesedcharacter_2)
          (else
            (`/Game/Blueprints/BP_TurorialCharacter.BeginRun` _poseesedcharacter_2))))
      (:`else`)))
  (:`Completed`
    (goto _label_2)))

(event `EnhancedInput|/Game/Input/Actions/IA_Strafe`
  (params (ActionValue :type Boolean) (ElapsedSeconds :type "Float (double-precision)") (TriggeredSeconds :type "Float (double-precision)") (InputAction :type "InputAction Object Reference" :default "/Game/Input/Actions/IA_Strafe.IA_Strafe"))
  (:`Started`
    (bind _poseesedcharacter (`self.PoseesedCharacter`)
      (:`then`
        (`/Game/Blueprints/BP_TurorialCharacter.BeginStrafe` _poseesedcharacter))
      (:`else`)))
  (:`Canceled`
    (bind _poseesedcharacter_2 (`self.PoseesedCharacter` :!label _label_3)
      (:`then`
        (`TurorialCharacter.BeginNeutral` _poseesedcharacter_2))
      (:`else`)))
  (:`Completed`
    (goto _label_3)))

(fn `UserConstructionScript`)
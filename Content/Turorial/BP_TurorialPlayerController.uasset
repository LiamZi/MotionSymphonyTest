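; Tutorial player controller that routes Enhanced Input actions to the possessed BP_TurorialCharacter.
; On possess, TryCacheCharacter casts the controlled pawn and caches it, and each input handler checks that reference is valid.
; Move forwards its value to the character's Move on triggered, canceled and completed, while Look adds yaw and pitch input.
; Jump only performs the validity check and has no action yet.
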(event `self.ReceivePossess`
  (params (PossessedPawn :type "Pawn Object Reference"))
  (`self.TryCacheCharacter`))

(event `EnhancedInput|/Game/Input/Actions/IA_Move`
  (params (ActionValue :type "Vector2D Structure") (ElapsedSeconds :type "Float (double-precision)") (TriggeredSeconds :type "Float (double-precision)") (InputAction :type "InputAction Object Reference" :default "/Game/Input/Actions/IA_Move.IA_Move"))
  (:`Triggered`
    (bind _poseesedcharacter (`self.PoseesedCharacter` :!label _label)
      (:`then`
        (`/Game/Turorial/BP_TurorialCharacter.Move` _poseesedcharacter ActionValue))
      (:`else`)))
  (:`Canceled`
    (goto _label))
  (:`Completed`
    (goto _label)))

(event `EnhancedInput|/Game/Input/Actions/IA_Look`
  (params (ActionValue :type "Vector2D Structure") (ElapsedSeconds :type "Float (double-precision)") (TriggeredSeconds :type "Float (double-precision)") (InputAction :type "InputAction Object Reference" :default "/Game/Input/Actions/IA_Look.IA_Look"))
  (:`Triggered`
    (bind _poseesedcharacter (`self.PoseesedCharacter`)
      (:`then`
        (`Pawn.AddControllerYawInput` _poseesedcharacter ActionValue_X)
        (`Pawn.AddControllerPitchInput` _poseesedcharacter ActionValue_Y))
      (:`else`))))

(event `EnhancedInput|/Game/Input/Actions/IA_Jump`
  (params (ActionValue :type Boolean) (ElapsedSeconds :type "Float (double-precision)") (TriggeredSeconds :type "Float (double-precision)") (InputAction :type "InputAction Object Reference" :default "/Game/Input/Actions/IA_Jump.IA_Jump"))
  (:`Triggered`
    (`self.PoseesedCharacter`
      (:`then`)
      (:`else`))))

(fn `UserConstructionScript`)
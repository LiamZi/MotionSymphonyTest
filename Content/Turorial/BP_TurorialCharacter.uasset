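; Tutorial player character with trajectory-driven locomotion, using camera-relative movement and Enhanced Input mapping swapped on controller change.
; Move feeds the TrajectoryGenerator, while Tick applies trajectory error warping during input and updates camera-based strafe direction.
; Style and speed functions set gameplay tags, generator tuning and warp modes, starting in Neutral Run.
; Tick calls root motion toggles by falling state, but both select no extraction.
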(event `self.ReceiveControllerChanged`
  (params (OldController :type "Controller Object Reference") (NewController :type "Controller Object Reference"))
  (`self.Remove Input Mapping` OldController)
  (`self.Add Input Mapping` NewController))

(event `self.ReceiveBeginPlay`
  (`self.BeginNeutral`)
  (`self.BeginRun`))

(event `self.ReceiveTick`
  (params (DeltaSeconds :type "Float (single-precision)"))
  (bind _returnvalue (`NavMovementComponent.IsFalling` (`self.CharacterMovement`)))
  (`|ExecutionSequence`
    (:`then_0`
      (bind _returnvalue_2 (`TrajectoryGenerator_Base.HasMoveInput` (`self.TrajectoryGenerator`)))
      (if _returnvalue_2
        (`TrajectoryErrorWarping.ApplyTrajectoryErrorWarping` (`self.TrajectoryErrorWarping`) DeltaSeconds 1.0)))
    (:`then_1`
      (if (`|EnumEquality` (`TrajectoryGenerator.TrajectoryBehaviour` (`self.TrajectoryGenerator`)) "Strafe")
        (`TrajectoryGenerator.SetStrafeDirectionFromCamera` (`self.TrajectoryGenerator`) (`self.Camera`))))
    (:`then_2`
      (if (`self.UseRootMotion`)
        (if _returnvalue
          (`self.DisableRootMotion`))
        (elif (not _returnvalue)
          (`self.EnableRootMotion`))))))

(fn `Add Input Mapping`
  (params (Controller :type "Controller Object Reference"))
  (`/Engine/EditorBlueprintResources/StandardMacros.IsValid` Controller
    (:`Is Valid`
      (if (`Controller.IsLocalPlayerController` Controller)
        (bind _asbp_turorial_player_controller (cast `/Game/Turorial/BP_TurorialPlayerController` Controller))
        (`EnhancedInputSubsystemInterface.AddMappingContext` (pcsubsystem `EnhancedInputLocalPlayerSubsystem` _asbp_turorial_player_controller) (`self.InputMapping`) 0 (struct))))))

(fn `BeginNeutral`
  (`self.SetStyleTag` (struct :`TagName` "Motion.Sytle.Neutral"))
  (set `TrajectoryGenerator.TrajectoryBehaviour` "Standard" (`self.TrajectoryGenerator`))
  (`TrajectoryErrorWarping.SetMode` (`self.TrajectoryErrorWarping`) "Standard" 60.0 50.0 0.25 30.0))

(fn `BeginRun`
  (bind _trajectorygenerator (`self.TrajectoryGenerator`))
  (`self.SetSpeedTag` (struct :`TagName` "Motion.Speed.Run"))
  (set `TrajectoryGenerator.MaxSpeed` 475.0 _trajectorygenerator)
  (set `TrajectoryGenerator.MoveResponse` 0.0 _trajectorygenerator)
  (set `TrajectoryGenerator.TurnResponse` 0.0 _trajectorygenerator)
  (set `self.NeutralCalibration` null))

(fn `BeginSprint`
  (bind _trajectorygenerator (`self.TrajectoryGenerator`))
  (if true
    (`self.SetSpeedTag` (struct))
    (set `TrajectoryGenerator.MaxSpeed` 650.0 _trajectorygenerator)
    (set `TrajectoryGenerator.MoveResponse` 6.0 _trajectorygenerator)
    (set `TrajectoryGenerator.TurnResponse` 10.0 _trajectorygenerator)
    (set `self.OverrideQualityVsResponsiveness` 0.45)
    (set `self.NeutralCalibration` null)))

(fn `BeginStrafe`
  (`self.SetStyleTag` (struct))
  (if (== (`self.SpeedTag`) (struct :`TagName` "Motion.Speed.Sprint"))
    (`self.BeginRun`))
  (set `TrajectoryGenerator.TrajectoryBehaviour` "Strafe" (`self.TrajectoryGenerator`))
  (`TrajectoryErrorWarping.SetMode` (`self.TrajectoryErrorWarping`) "Strafe" 90.0 50.0 2.0 180.0))

(fn `BeginWalk`
  (bind _trajectorygenerator (`self.TrajectoryGenerator`))
  (`self.SetSpeedTag` (struct :`TagName` "Motion.Speed.Walk"))
  (set `TrajectoryGenerator.MaxSpeed` 215.0 _trajectorygenerator)
  (set `TrajectoryGenerator.MoveResponse` 9.0 _trajectorygenerator)
  (set `TrajectoryGenerator.TurnResponse` 8.0 _trajectorygenerator)
  (set `self.OverrideQualityVsResponsiveness` 0.5))

(fn `DisableRootMotion`
  (bind _returnvalue (`SkeletalMeshComponent.GetAnimInstance` (`self.Mesh`)))
  (`/Engine/EditorBlueprintResources/StandardMacros.IsValid` _returnvalue
    (:`Is Valid`
      (`AnimInstance.SetRootMotionMode` _returnvalue "NoRootMotionExtraction")
      (set `self.UseRootMotion` false))))

(fn `EnableRootMotion`
  (bind _returnvalue (`SkeletalMeshComponent.GetAnimInstance` (`self.Mesh`)))
  (`/Engine/EditorBlueprintResources/StandardMacros.IsValid` _returnvalue
    (:`Is Valid`
      (`AnimInstance.SetRootMotionMode` _returnvalue "NoRootMotionExtraction")
      (set `self.UseRootMotion` false))))

(fn `Move`
  (params (`Input X` :type "Float (double-precision)") (`Input Y` :type "Float (double-precision)"))
  (bind _returnvalue (`MMBlueprintFunctionLibrary.GetVectorRelativeToCamera` `Input Y` `Input X` (`self.Camera`)))
  (`self.AddMovementInput` _returnvalue)
  (`TrajectoryGenerator_Base.SetTrajectoryInput` (`self.TrajectoryGenerator`) (.x _returnvalue) (.y _returnvalue) 0.0))

(fn `Remove Input Mapping`
  (params (Controller :type "Controller Object Reference"))
  (locals (NewLocalVar :type "InputMappingContext Object Reference"))
  (`/Engine/EditorBlueprintResources/StandardMacros.IsValid` Controller
    (:`Is Valid`
      (if (`Controller.IsLocalPlayerController` Controller)
        (bind _asbp_turorial_player_controller (cast `/Game/Turorial/BP_TurorialPlayerController` Controller))
        (bind _returnvalue (pcsubsystem `EnhancedInputLocalPlayerSubsystem` _asbp_turorial_player_controller))
        (`/Engine/EditorBlueprintResources/StandardMacros.IsValid` _returnvalue
          (:`Is Valid`
            (`EnhancedInputSubsystemInterface.RemoveMappingContext` _returnvalue (`self.InputMapping`) (struct))))))))

(fn `SetSpeedTag`
  (params (SpeedTag :type "GameplayTag Structure"))
  (`BlueprintGameplayTagLibrary.RemoveGameplayTag` (`self.Locomotion Tags`) (`self.SpeedTag`))
  (bind _output_get (set `self.SpeedTag` SpeedTag))
  (`BlueprintGameplayTagLibrary.AddGameplayTag` (`self.Locomotion Tags`) _output_get))

(fn `SetStyleTag`
  (params (StyleTag :type "GameplayTag Structure"))
  (`BlueprintGameplayTagLibrary.RemoveGameplayTag` (`self.Locomotion Tags`) (`self.StyleTag`))
  (bind _output_get (set `self.StyleTag` StyleTag))
  (`BlueprintGameplayTagLibrary.AddGameplayTag` (`self.Locomotion Tags`) _output_get))

(fn `UndoModelRotation`)

(fn `UserConstructionScript`)
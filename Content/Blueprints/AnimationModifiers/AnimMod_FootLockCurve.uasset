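; Animation modifier that bakes FootSpeed_L and FootSpeed_R curves into an animation sequence from toe bone motion, and removes them on revert.
; It steps through the sequence at an assumed 30 fps, sampling world-space pose locations of both toes at the previous and next frames.
; Each key stores that central-difference distance multiplied, not divided, by the time span, so values are not true speeds.
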(event `self.OnRevert`
  (params (AnimationSequence :type "AnimSequence Object Reference"))
  (`self.RemoveCurves` AnimationSequence))

(event `self.OnApply`
  (params (AnimationSequence :type "AnimSequence Object Reference"))
  (`|ExecutionSequence`
    (:`then_0`
      ;[1 0.892 0] Initialization
      (`self.InitializeCurves` AnimationSequence)
      (set `self.FrameDelta` (/ 1.0 30.0)))
    (:`then_1`
      ;[1 0.892 0] Loop through every frame, calculate speed and add curves keys
      (for _index (range (+ (`KismetMathLibrary.FTrunc` (/ (`AnimationAsset.GetPlayLength` AnimationSequence) (`self.FrameDelta`))) 1))
        (`self.EvaluateFrame` AnimationSequence _index)))))

(fn `EvaluateFrame`
  (params (Sequence :type "AnimSequence Object Reference") (FrameIndex :type Integer))
  (locals (StartFrame :type Integer) (EndFrame :type Integer) (StartLocation_L :type "Vector Structure") (EndLocation_L :type "Vector Structure") (StartLocation_R :type "Vector Structure") (EndLocation_R :type "Vector Structure") (Time :type "Float (double-precision)"))
  (bind _returnvalue (* (`self.FrameDelta`) (- (`local.EndFrame`) (`local.StartFrame`))))
  (set `local.Time` (* FrameIndex (`self.FrameDelta`)))
  (`|ExecutionSequence`
    (:`then_0`
      ;[1 0.832 0] Evaluate and record Left and Right toe locations at the previous frame
      (bind _output_get (set `local.StartFrame` (`KismetMathLibrary.Clamp` (- FrameIndex 1) 0 (`AnimationBlueprintLibrary.GetNumFrames` Sequence))))
      (bind _pose (`AnimPoseExtensions.GetAnimPoseAtFrame` Sequence _output_get (`self.Evaluation Options`)))
      (bind _returnvalue_location (`KismetMathLibrary.BreakTransform` (`AnimPoseExtensions.GetBonePose` _pose (`self.ToeName_L`) "World")))
      (set `local.StartLocation_L` _returnvalue_location)
      (bind _returnvalue_location_2 (`KismetMathLibrary.BreakTransform` (`AnimPoseExtensions.GetBonePose` _pose (`self.ToeName_R`) "World")))
      (set `local.StartLocation_R` _returnvalue_location_2))
    (:`then_1`
      ;[1 0.832 0] Evaluate and record Left and Right toe locations at the next frame
      (bind _output_get_2 (set `local.EndFrame` (`KismetMathLibrary.Clamp` (+ FrameIndex 1) 0 (`AnimationBlueprintLibrary.GetNumFrames` Sequence))))
      (bind _pose_2 (`AnimPoseExtensions.GetAnimPoseAtFrame` Sequence _output_get_2 (`self.Evaluation Options`)))
      (bind _returnvalue_location_3 (`KismetMathLibrary.BreakTransform` (`AnimPoseExtensions.GetBonePose` _pose_2 (`self.ToeName_L`) "World")))
      (set `local.EndLocation_L` _returnvalue_location_3)
      (bind _returnvalue_location_4 (`KismetMathLibrary.BreakTransform` (`AnimPoseExtensions.GetBonePose` _pose_2 (`self.ToeName_R`) "World")))
      (set `local.EndLocation_R` _returnvalue_location_4))
    (:`then_2`
      ;[1 0.832 0] Calculate the average speed of the left and right foot this frame and add these values as keys to the curve
      (`AnimationBlueprintLibrary.AddFloatCurveKey` Sequence "FootSpeed_L" (`local.Time`) (* (`KismetMathLibrary.VSize` (- (`local.EndLocation_L`) (`local.StartLocation_L`))) _returnvalue))
      (`AnimationBlueprintLibrary.AddFloatCurveKey` Sequence "FootSpeed_R" (`local.Time`) (* (`KismetMathLibrary.VSize` (- (`local.EndLocation_R`) (`local.StartLocation_R`))) _returnvalue)))))

(fn `InitializeCurves`
  (params (AnimationSequence :type "AnimSequence Object Reference"))
  (`AnimationBlueprintLibrary.AddCurve` AnimationSequence "FootSpeed_L")
  (`AnimationBlueprintLibrary.AddCurve` AnimationSequence "FootSpeed_R"))

(fn `RemoveCurves`
  (params (Sequence :type "AnimSequence Object Reference"))
  (`AnimationBlueprintLibrary.RemoveCurve` Sequence "FootSpeed_L")
  (`AnimationBlueprintLibrary.RemoveCurve` Sequence "FootSpeed_R"))
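; Player character driven by trajectory-based motion animation, with walk, run, sprint and strafe locomotion modes.
; Camera-relative input feeds movement and the TrajectoryGenerator, with a multicast event applying it on non-local instances.
; Mode functions set gameplay tags and tune trajectory speed and response; strafe follows the camera and disallows sprint.
; Tick applies trajectory error warping during input and switches off full root motion while falling.
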(event `self.ReceiveBeginPlay`
  (`self.BeginNeutral`)
  (`self.BeginRun`))

(event `self.ReceiveTick`
  (params (DeltaSeconds :type "Float (single-precision)"))
  (bind _returnvalue (`NavMovementComponent.IsFalling` (`self.CharacterMovement`)))
  (`|ExecutionSequence`
    (:`then_0`
      (bind _returnvalue_2 (`TrajectoryGenerator_Base.HasMoveInput` (`self._trajectoryGenerator`)))
      (if _returnvalue_2
        (`TrajectoryErrorWarping.ApplyTrajectoryErrorWarping` (`self.BP_TrajectoryErrorWarping`) DeltaSeconds 1.0)))
    (:`then_1`
      (if (`|EnumEquality` (`TrajectoryGenerator.TrajectoryBehaviour` (`self._trajectoryGenerator`)) "Strafe")
        (`TrajectoryGenerator.SetStrafeDirectionFromCamera` (`self._trajectoryGenerator`) (`self.Camera`))))
    (:`then_2`
      (if (`self.UseRootMotion`)
        (if _returnvalue
          (`self.DisableRootMotion`))
        (elif (not _returnvalue)
          (`self.EnableRootMotion`))))))

(event `OnSetTrajectoryInputVector_Multicast`
  (params (X :type "Float (double-precision)") (Y :type "Float (double-precision)"))
  (if (not (`self.IsLocallyControlled`))
    (`TrajectoryGenerator_Base.SetTrajectoryInput` (`self._trajectoryGenerator`) X Y 0.0)))

(fn `BeginRun`
  (bind __trajectorygenerator (`self._trajectoryGenerator`))
  (`self.BP_SetSpeedTag` (struct :`TagName` "Motion.Speed.Run"))
  (set `TrajectoryGenerator.MaxSpeed` 475.0 __trajectorygenerator)
  (set `TrajectoryGenerator.MoveResponse` 8.0 __trajectorygenerator)
  (set `TrajectoryGenerator.TurnResponse` 12.0 __trajectorygenerator)
  (set `self.OverrideQualityVsResponsiveness` 0.5)
  (set `self.NeutralCalibration` null))

(fn `BeginSprint`
  (bind __trajectorygenerator (`self._trajectoryGenerator`))
  (if (!= (`self.BP_StyleTag`) (struct :`TagName` "Motion.Sytle.Strafe"))
    (`self.BP_SetSpeedTag` (struct :`TagName` "Motion.Speed.Sprint"))
    (set `TrajectoryGenerator.MaxSpeed` 650.0 __trajectorygenerator)
    (set `TrajectoryGenerator.MoveResponse` 6.0 __trajectorygenerator)
    (set `TrajectoryGenerator.TurnResponse` 10.0 __trajectorygenerator)
    (set `self.OverrideQualityVsResponsiveness` 0.45)
    (set `self.NeutralCalibration` null)))

(fn `BeginStrafe`
  (`self.SetStyleTag` (struct :`TagName` "Motion.Sytle.Strafe"))
  (if (== (`self.BP_SpeedTag`) (struct :`TagName` "Motion.Speed.Sprint"))
    (`self.BeginRun`))
  (set `TrajectoryGenerator.TrajectoryBehaviour` "Strafe" (`self._trajectoryGenerator`))
  (`TrajectoryErrorWarping.SetMode` (`self.BP_TrajectoryErrorWarping`) "Strafe" 90.0 50.0 2.0 180.0))

(fn `BeginWalk`
  (bind __trajectorygenerator (`self._trajectoryGenerator`))
  (`self.BP_SetSpeedTag` (struct :`TagName` "Motion.Speed.Walk"))
  (set `TrajectoryGenerator.MaxSpeed` 215.0 __trajectorygenerator)
  (set `TrajectoryGenerator.MoveResponse` 9.0 __trajectorygenerator)
  (set `TrajectoryGenerator.TurnResponse` 8.0 __trajectorygenerator)
  (set `self.OverrideQualityVsResponsiveness` 0.5))

(fn `BP_Add Input Mapping`
  (params (Controller :type "Controller Object Reference"))
  (`/Engine/EditorBlueprintResources/StandardMacros.IsValid` Controller
    (:`Is Valid`
      (if (`Controller.IsLocalPlayerController` Controller)
        (bind _asbp_turorial_player_controller (cast `/Game/Controller/BP_TurorialPlayerController` Controller))
        (`EnhancedInputSubsystemInterface.AddMappingContext` (pcsubsystem `EnhancedInputLocalPlayerSubsystem` _asbp_turorial_player_controller) (`self.InputMapping`) 0 (struct))))))

(fn `BP_SetSpeedTag`
  (params (SpeedTag :type "GameplayTag Structure"))
  (`BlueprintGameplayTagLibrary.RemoveGameplayTag` (`self.BP_Locomotion Tags`) (`self.BP_SpeedTag`))
  (bind _output_get (set `self.BP_SpeedTag` SpeedTag))
  (`BlueprintGameplayTagLibrary.AddGameplayTag` (`self.BP_Locomotion Tags`) _output_get))

(fn `DisableRootMotion`
  (bind _returnvalue (`SkeletalMeshComponent.GetAnimInstance` (`self.Mesh`)))
  (`/Engine/EditorBlueprintResources/StandardMacros.IsValid` _returnvalue
    (:`Is Valid`
      (`AnimInstance.SetRootMotionMode` _returnvalue "RootMotionFromMontagesOnly")
      (set `self.UseRootMotion` false))))

(fn `EnableRootMotion`
  (bind _returnvalue (`SkeletalMeshComponent.GetAnimInstance` (`self.Mesh`)))
  (`/Engine/EditorBlueprintResources/StandardMacros.IsValid` _returnvalue
    (:`Is Valid`
      (`AnimInstance.SetRootMotionMode` _returnvalue "RootMotionFromEverything")
      (set `self.UseRootMotion` true))))

(fn `Move`
  (params (InputVector :type "Vector2D Structure"))
  (bind _returnvalue (`MMBlueprintFunctionLibrary.GetVectorRelativeToCamera` InputVector_Y InputVector_X (`self.Camera`)))
  (`self.AddMovementInput` _returnvalue)
  (`TrajectoryGenerator_Base.SetTrajectoryInput` (`self._trajectoryGenerator`) (.x _returnvalue) (.y _returnvalue) 0.0))

(fn `Remove Input Mapping`
  (params (Controller :type "Controller Object Reference"))
  (locals (NewLocalVar :type "InputMappingContext Object Reference"))
  (`/Engine/EditorBlueprintResources/StandardMacros.IsValid` Controller
    (:`Is Valid`
      (if (`Controller.IsLocalPlayerController` Controller)
        (bind _asbp_turorial_player_controller (cast `/Game/Controller/BP_TurorialPlayerController` Controller))
        (bind _returnvalue (pcsubsystem `EnhancedInputLocalPlayerSubsystem` _asbp_turorial_player_controller))
        (`/Engine/EditorBlueprintResources/StandardMacros.IsValid` _returnvalue
          (:`Is Valid`
            (`EnhancedInputSubsystemInterface.RemoveMappingContext` _returnvalue (`self.InputMapping`) (struct))))))))

(fn `UndoModelRotation`
  (bind (_returnvalue_roll _returnvalue_pitch _returnvalue_yaw) (`KismetMathLibrary.BreakRotator` (`KismetMathLibrary.NormalizedDeltaRotator` (`self.K2_GetActorRotation`) (`self.LastFrameRotation`))))
  (`SceneComponent.K2_AddLocalRotation` (`self.Mesh`) (`KismetMathLibrary.NegateRotator` (`KismetMathLibrary.MakeRotator` 0.0 0.0 _returnvalue_yaw)) false false)
  (set `self.LastFrameRotation` (`self.K2_GetActorRotation`))
  (return))

(fn `UserConstructionScript`)